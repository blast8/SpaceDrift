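; BP_SelectionCharacter is the preview actor for the selection menu, showing a rotating ship that can be switched.
; ChangeShip advances through the Ships array, wrapping to the first entry, and applies the result to the skeletal mesh.
; It then stores that mesh in GI_Selection, the game instance, as the selected ship.
; Tick spins the mesh by a fixed yaw step each frame, independent of delta time.
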(event `Change Ship`
  (bind _output (`|GetArrayItem` (`self.Ships`) (`self.currentShipIndex`)))
  (if (< (`self.currentShipIndex`) (- (`KismetArrayLibrary.Array_Length` (`self.Ships`)) 1))
    (`/Engine/EditorBlueprintResources/StandardMacros.IncrementInt` (`self.currentShipIndex`)
      (:`  `
        _))
    (else
      (set `self.currentShipIndex` 0)))
  (`SkeletalMeshComponent.SetSkeletalMeshAsset` (`self.Mesh`) _output)
  (bind _asgi_selection (cast `/Game/Selection_Menu/GI_Selection` (`GameplayStatics.GetGameInstance`)))
  (set `/Game/Selection_Menu/GI_Selection.skeletalMeshSelected` _output _asgi_selection))

(event `self.ReceiveTick`
  (params (DeltaSeconds :type "Float (single-precision)"))
  (`SceneComponent.K2_AddLocalRotation` (`self.Mesh`) (struct :`Yaw` 0.4) false false))

(fn `UserConstructionScript`)