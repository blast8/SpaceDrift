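; BP_Test is an opponent pawn that patrols the level's TargetPoint actors and is destroyed when its HealthSystem reports death.
; BeginPlay gathers every TargetPoint into an array, in the order GetAllActorsOfClass returns them.
; Each Tick feeds a normalized direction to the current point into AddMovementInput, with no pathfinding.
; Within a small distance threshold it advances the index, wrapping around to loop indefinitely.
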(event `self.ReceiveTick`
  (params (DeltaSeconds :type "Float (single-precision)"))
  (bind _returnvalue (- (`self.K2_GetActorLocation` (`|GetArrayItem` (`self.Target points`) (`self.TargetIndex`))) (`self.K2_GetActorLocation`)))
  ; Move To Current Point (Tick): if array has points, compute direction and move pawn
  (bind _returnvalue_2 (`KismetArrayLibrary.Array_Length` (stale `self.ReceiveBeginPlay` _output_get)))
  (if (> _returnvalue_2 0)
    ;; Reached Point -> Next Index: when distance < 100, TargetIndex = (TargetIndex + 1) % PointsCount
    (`self.AddMovementInput` (`KismetMathLibrary.Normal` _returnvalue))
    (if (< (`KismetMathLibrary.VSize` _returnvalue) 100.0)
      (set `self.TargetIndex` (mod (+ (`self.TargetIndex`) 1) _returnvalue_2)))))

(event `self.ReceiveBeginPlay`
  ; Move To Current Point (Tick): if array has points, compute direction and move pawn
  ;; Init Path Points (BeginPlay): find all TargetPoint actors, save to array, set start index = 0
  (bind _outactors (`GameplayStatics.GetAllActorsOfClass` "/Script/Engine.TargetPoint"))
  (bind _output_get (set `self.Target points` _outactors))
  (set `self.TargetIndex` 0))

(event `self.HealthSystem.OnDeath`
  ; Move To Current Point (Tick): if array has points, compute direction and move pawn
  (`self.K2_DestroyActor`))

(fn `UserConstructionScript`)