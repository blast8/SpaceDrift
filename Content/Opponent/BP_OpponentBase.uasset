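; Base opponent that travels a looping route through all TargetPoint actors in the level while steering around obstacles.
; Each tick it moves via movement input, smoothly rotates toward the current target and line-traces ahead for obstacles.
; When blocked, it sphere-sweeps from the hit point toward right, left, up and down offsets, steering to the first clear one, with down as fallback.
; Traces draw debug shapes.
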(event `self.ReceiveTick`
  (params (DeltaSeconds :type "Float (single-precision)"))
  (`self.MoveToFunction`)
  (`self.RotateTowardTarget`)
  (`self.DetectObstacle`))

(event `self.ReceiveBeginPlay`
  (`self.GetTargetIndex`))

(fn `DetectObstacle`
  (bind _returnvalue (`self.K2_GetActorLocation`))
  (bind (_outhit _returnvalue_2) (`KismetSystemLibrary.LineTraceSingle` :`Start` _returnvalue :`End` (+ _returnvalue (* (`self.GetActorForwardVector`) 500.0)) :`TraceChannel` "TraceTypeQuery1" :`DrawDebugType` "ForDuration" :`DrawTime` 3.0))
  (set `self.ObstacleDetected` _returnvalue_2)
  (bind _output_get (set `self.ObstacleHitLocation` (`.ImpactPoint` (`GameplayStatics.BreakHitResult` _outhit))))
  (`KismetSystemLibrary.SphereTraceSingle` :`Start` _output_get :`End` _output_get :`Radius` 150.0 :`TraceChannel` "TraceTypeQuery1" :`DrawDebugType` "ForDuration"))

(fn `FindAvoidancePoint`
  (bind _returnvalue (`self.GetTransform`))
  (bind _obstaclehitlocation (`self.ObstacleHitLocation`))
  (bind _returnvalue_2 (`KismetMathLibrary.TransformLocation` _returnvalue (800.0 800.0 0.0)))
  (bind _returnvalue_3 (`KismetMathLibrary.TransformLocation` _returnvalue (800.0 -800.0 0.0)))
  (bind _returnvalue_4 (`KismetMathLibrary.TransformLocation` _returnvalue (800.0 0.0 800.0)))
  (bind _returnvalue_5 (`KismetMathLibrary.TransformLocation` _returnvalue (800.0 0.0 -800.0)))
  (bind (_outhits _returnvalue_6) (`KismetSystemLibrary.SphereTraceMulti` :`Start` _obstaclehitlocation :`End` _returnvalue_2 :`Radius` 120.0 :`TraceChannel` "TraceTypeQuery1" :`DrawDebugType` "ForDuration" :`DrawTime` 2.0))
  (if _returnvalue_6
    (bind (_outhits_2 _returnvalue_7) (`KismetSystemLibrary.SphereTraceMulti` :`Start` _obstaclehitlocation :`End` _returnvalue_3 :`Radius` 120.0 :`TraceChannel` "TraceTypeQuery1" :`DrawDebugType` "ForDuration" :`DrawTime` 2.0))
    (if _returnvalue_7
      (bind (_outhits_3 _returnvalue_8) (`KismetSystemLibrary.SphereTraceMulti` :`Start` _obstaclehitlocation :`End` _returnvalue_4 :`Radius` 120.0 :`TraceChannel` "TraceTypeQuery1" :`DrawDebugType` "ForDuration" :`DrawTime` 2.0))
      (if _returnvalue_8
        (bind (_outhits_4 _returnvalue_9) (`KismetSystemLibrary.SphereTraceMulti` :`Start` _obstaclehitlocation :`End` _returnvalue_5 :`Radius` 120.0 :`TraceChannel` "TraceTypeQuery1" :`DrawDebugType` "ForDuration" :`DrawTime` 2.0))
        (if _returnvalue_9
          _
          (else
            _))
        (set `self.AvoidancePoint` _returnvalue_5)
        (else
          (set `self.AvoidancePoint` _returnvalue_4)))
      (else
        (set `self.AvoidancePoint` _returnvalue_3)))
    (else
      (set `self.AvoidancePoint` _returnvalue_2))))

(fn `GetTargetIndex`
  (bind _outactors (`GameplayStatics.GetAllActorsOfClass` "/Script/Engine.TargetPoint"))
  (bind _output_get (set `self.Target points` _outactors))
  (set `self.Target Index` 0)
  (set `self.InitialIndex` (`KismetArrayLibrary.Array_Length` _output_get))
  (return))

(fn `MoveToFunction`
  (bind _target_points (`self.Target points`))
  (bind _returnvalue (`KismetArrayLibrary.Array_Length` _target_points))
  (bind _returnvalue_2 (- (`self.K2_GetActorLocation` (`|GetArrayItem` _target_points (`self.Target Index`))) (`self.K2_GetActorLocation`)))
  (if (`self.ObstacleDetected`)
    (`self.FindAvoidancePoint`)
    (`self.AddMovementInput` (`KismetMathLibrary.GetForwardVector` (`KismetMathLibrary.FindLookAtRotation` (`self.K2_GetActorLocation`) (`self.AvoidancePoint`))))
    (elif (> _returnvalue 0)
      (`self.AddMovementInput` (`KismetMathLibrary.Normal` _returnvalue_2))
      (if (< (`KismetMathLibrary.VSize` _returnvalue_2) 100.0)
        (set `self.Target Index` (mod (+ (`self.Target Index`) 1) _returnvalue))))))

(fn `RotateTowardTarget`
  (`self.K2_SetActorRotation` (`KismetMathLibrary.RInterpTo` (`self.K2_GetActorRotation`) (`KismetMathLibrary.FindLookAtRotation` (`self.K2_GetActorLocation`) (`self.K2_GetActorLocation` (`|GetArrayItem` (`self.Target Points`) (`self.Target Index`)))) (`GameplayStatics.GetWorldDeltaSeconds`) 3.0)))

(fn `UserConstructionScript`)