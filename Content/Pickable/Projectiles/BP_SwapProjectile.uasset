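; BP_SwapProjectile is a seeking projectile that triggers a swap between the pawn that fired it and the actor it hits.
; On BeginPlay it stores its owning pawn as shooter and targets the first other WorldStatic actor found within a search radius, not necessarily the nearest.
; Tick turns it toward that target.
; Overlapping a non-shooter BPI_ShipEffect implementer sends that actor SwapWith, passing the shooter, then destroys the projectile.
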(event `self.ReceiveBeginPlay`
  (bind _aspawn (cast `Pawn` (`self.GetOwner`)))
  (set `self.ShooterPawn` _aspawn)
  (bind _outactors (`KismetSystemLibrary.SphereOverlapActors` (`self.K2_GetActorLocation`) (`self.SearchRadius`) (`|MakeArray` "ObjectTypeQuery1" :!type "EObjectTypeQuery Enum")))
  (for _array_element _outactors
    (if (!= _array_element (`self.ShooterPawn`))
      (set `self.TargetActor` _array_element)
      (break))))

(event `self.ReceiveActorBeginOverlap`
  (params (OtherActor :type "Actor Object Reference"))
  (if (!= OtherActor (`self.ShooterPawn`))
    (if (`KismetSystemLibrary.DoesImplementInterface` OtherActor "/Game/Pickable/BPI_ShipEffect.BPI_ShipEffect_C")
      (message `/Game/Pickable/BPI_ShipEffect.SwapWith` OtherActor (`self.ShooterPawn`))
      (`self.K2_DestroyActor`))))

(event `self.ReceiveTick`
  (params (DeltaSeconds :type "Float (single-precision)"))
  (bind _targetactor (`self.TargetActor`))
  (`/Engine/EditorBlueprintResources/StandardMacros.IsValid` _targetactor
    (:`Is Valid`
      (`self.K2_SetActorRotation` (`KismetMathLibrary.FindLookAtRotation` (`self.K2_GetActorLocation`) (`self.K2_GetActorLocation` _targetactor))))))

(fn `UserConstructionScript`)