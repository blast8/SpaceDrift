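; BP_BlackHoleProjectile is a pickable-weapon projectile that acts as a black hole, applying a gravity pull to ships.
; On BeginPlay it sets its lifespan to the effect duration and sizes the GravityZone sphere to the gravity radius.
; Overlapping actors that implement BPI_ShipEffect receive a one-time gravity pull message per overlap, carrying the black hole's location, intensity and full effect duration.
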(event `self.ReceiveBeginPlay`
  (`self.SetLifeSpan` (`self.EffectDuration`))
  (`SphereComponent.SetSphereRadius` (`self.GravityZone`) (`self.GravityRadius`) true))

(event `self.ReceiveActorBeginOverlap`
  (params (OtherActor :type "Actor Object Reference"))
  (if (`KismetSystemLibrary.DoesImplementInterface` OtherActor "/Game/Pickable/BPI_ShipEffect.BPI_ShipEffect_C")
    (message `/Game/Pickable/BPI_ShipEffect.ApplyGravityPull` OtherActor (`self.K2_GetActorLocation`) (`self.GravityIntensity`) (`self.EffectDuration`))))

(fn `UserConstructionScript`)