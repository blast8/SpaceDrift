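; BP_Collectible is a pickable actor that grants a random bonus to an actor that overlaps it.
; On overlap it rolls one of five bonuses, fetches a component from the other actor and casts it to BC_BonusHolder.
; If that succeeds, it passes the zero-based bonus index to PickupBonus and destroys itself.
; The component lookup uses the generic ActorComponent class, and GetBonusInfo returns only an empty name.
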(event `self.ReceiveActorBeginOverlap`
  (params (OtherActor :type "Actor Object Reference"))
  (bind _returnvalue (`self.GetComponentByClass` OtherActor "/Script/Engine.ActorComponent"))
  (bind _bonusid (`self.GetRandomBonus`))
  (`/Engine/EditorBlueprintResources/StandardMacros.IsValid` _returnvalue
    (:`Is Valid`
      (bind _asbc_bonus_holder (cast `/Game/Pickable/Components/BC_BonusHolder` _returnvalue))
      (`/Game/Pickable/Components/BC_BonusHolder.PickupBonus` _asbc_bonus_holder (- _bonusid 1))
      (`self.K2_DestroyActor`))))

(fn `GetBonusInfo`
  (returns (BonusName :type String) (BonusIcon :type "Texture2D Object Reference"))
  (return "" null))

(fn `GetRandomBonus`
  (returns (BonusID :type Integer))
  (return (`KismetMathLibrary.RandomIntegerInRange` 1 5)))

(fn `UserConstructionScript`)