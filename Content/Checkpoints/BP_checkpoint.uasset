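; BP_checkpoint is an ordered checkpoint that tracks an overlapping actor's progress along a course and can act as the finish.
; On sphere overlap, it casts the actor and compares its own Index to that actor's crossed count plus one.
; A match updates the count and last checkpoint, plays a pass sound and calls Finish if flagged.
; Skipped or repeated checkpoints only print a message and trigger sound playback.
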(event `self.Sphere.OnComponentBeginOverlap`
  (params (OverlappedComponent :type "PrimitiveComponent Object Reference") (OtherActor :type "Actor Object Reference") (OtherComp :type "PrimitiveComponent Object Reference") (OtherBodyIndex :type Integer) (bFromSweep :type Boolean) (SweepResult :type "HitResult Structure (by ref)"))
  (bind _index (`self.index`))
  (bind _asbp_jet_pawn (cast `` OtherActor))
  (`/Engine/EditorBlueprintResources/StandardMacros.CompareInt` _index (+ (`/Game/Checkpoints/BP_checkpoint.checkpointscrossed` _asbp_jet_pawn) 1)
    (:`>`
      (`KismetSystemLibrary.PrintString` "Youre missing a checkpoint")
      (`GameplayStatics.PlaySound2D` "/Game/Checkpoints/CheckpointFail.CheckpointFail" 1.0 1.0 0.0 null null))
    (:`==`
      (set `/Game/Checkpoints/BP_checkpoint.checkpointscrossed` _index _asbp_jet_pawn)
      (set `/Game/Checkpoints/BP_checkpoint.lastcheckpoint` self _asbp_jet_pawn)
      (`GameplayStatics.PlaySound2D` "/Game/Checkpoints/CheckpointPass.CheckpointPass" 1.0 1.0 0.0 null null)
      (if (`self.isfinish`)
        (`self.finish` _asbp_jet_pawn)))
    (:`<`
      (`KismetSystemLibrary.PrintString` "Youve already been here")
      (`GameplayStatics.PlaySound2D` null 1.0 1.0 0.0 null null))))

(fn `UserConstructionScript`)