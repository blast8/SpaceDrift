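; Blueprint function library with a line-of-sight check that tells whether a pawn can detect the player.
; TracePlayer first tests that the player is within about 60 degrees of an arrow component's forward vector using a dot product.
; It then line-traces from the arrow toward the player against several object types, reporting whether the first hit is player character 0 and returning the impact point as ShipLocation.
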(fn `Trace Player`
  (params (Arrow :type "ArrowComponent Object Reference") (`Player Location` :type "Vector Structure") (`Pawn Location` :type "Vector Structure") (Pawn :type "Actor Object Reference"))
  (returns (`Player Found?` :type Boolean) (`Ship Location` :type "Vector Structure"))
  (locals (`Trace Distance` :type "Float (double-precision)" :default 3000.0))
  (bind _returnvalue (`KismetMathLibrary.Normal` (- `Player Location` `Pawn Location`)))
  (bind _returnvalue_2 (`SceneComponent.K2_GetComponentLocation` (`local.Arrow`)))
  (if (> (`KismetMathLibrary.Dot_VectorVector` (`SceneComponent.GetForwardVector` Arrow) _returnvalue) 0.5)
    (bind (_outhit _returnvalue_3) (`KismetSystemLibrary.LineTraceSingleForObjects` (`local.Pawn`) _returnvalue_2 (+ _returnvalue_2 (* _returnvalue (`local.Trace Distance`))) (`|MakeArray` "ObjectTypeQuery1" "ObjectTypeQuery2" "ObjectTypeQuery3" "ObjectTypeQuery4" "ObjectTypeQuery5" "ObjectTypeQuery6" :!type "EObjectTypeQuery Enum")))
    (if _returnvalue_3
      (bind (_bblockinghit _binitialoverlap _time _distance _location _impactpoint _normal _impactnormal _physmat _hitactor) (`GameplayStatics.BreakHitResult` _outhit))
      (return (== (`GameplayStatics.GetPlayerCharacter` null) _hitactor) _impactpoint)
      (else
        (return false (0.0 0.0 0.0))))))