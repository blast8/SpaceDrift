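; Turret actor that tracks the player pawn and fires a laser at it.
; BeginPlay caches the player pawn as the target; while it is valid, Tick sets Head's relative yaw and Gun's relative roll from the yaw and pitch of world-space look-at rotations.
; Each tick it also moves BPLaserComponent to a forward offset from the gun, matches the gun's rotation and calls Fire, with no range or cooldown check.
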(event `self.ReceiveBeginPlay`
  (set `self.TargetActor` (`GameplayStatics.GetPlayerPawn` 0)))

(event `self.ReceiveTick`
  (params (DeltaSeconds :type "Float (single-precision)"))
  (bind _head (`self.Head`))
  (bind _targetactor (`self.TargetActor`))
  (bind _gun (`self.Gun`))
  (bind _bp_lasercomponent (`self.BP_LaserComponent`))
  (bind _gun_2 (`self.Gun`))
  (bind _returnvalue (`self.K2_GetActorLocation` _targetactor))
  (if (`KismetSystemLibrary.IsValid` _targetactor)
    (`SceneComponent.K2_SetRelativeRotation` _head (`KismetMathLibrary.MakeRotator` 0.0 0.0 (.yaw (`KismetMathLibrary.FindLookAtRotation` (`SceneComponent.K2_GetComponentLocation` _head) _returnvalue))) false false)
    (`SceneComponent.K2_SetRelativeRotation` _gun (`KismetMathLibrary.MakeRotator` (.pitch (`KismetMathLibrary.FindLookAtRotation` (`SceneComponent.K2_GetComponentLocation` _gun) _returnvalue))) false false)
    (`SceneComponent.K2_SetWorldLocationAndRotation` _bp_lasercomponent (`KismetMathLibrary.TransformLocation` (`SceneComponent.K2_GetComponentToWorld` _gun_2) (`KismetMathLibrary.MakeVector` 200.0)) (`SceneComponent.K2_GetComponentRotation` _gun_2) false false)
    (`/Game/Jet/Blueprints/Components/BP_LaserComponent.Fire` _bp_lasercomponent)))

(fn `UserConstructionScript`)