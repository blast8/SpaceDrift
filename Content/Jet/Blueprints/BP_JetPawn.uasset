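; Player jet pawn with floating movement, turbo boost, a laser-beam fire effect, bonus use and a gravity pull.
; Movement input drives translation, while camera and roll inputs apply physics torque to JetFighter, with damped roll auto-leveling.
; Tick turns velocity into a smoothed Speed that scales engine flame and light, and updates spring-arm lag, length and boost FOV.
; A looping timer feeds Speed into the HUD's dynamic speedlines material.
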(event `self.ReceiveTick`
  (params (DeltaSeconds :type "Float (single-precision)"))
  (bind _returnvalue (`GameplayStatics.GetWorldDeltaSeconds`))
  (`self.SpringArmLengthInterpolation`)
  (`|ExecutionSequence`
    (:`then_0`
      (`self.Max Speed`)
      (bind _speedvalue (`self.CalculateSpeedState`))
      (`self.Flame intensity` _speedvalue))
    (:`then_1`
      (`self.CameraFollowWithLag` _returnvalue)
      (`self.AutoLevelRoll` _returnvalue))
    (:`then_2`
      (if (`self.bGravityPull`)
        (`self.AddMovementInput` self (`KismetMathLibrary.Vector_NormalUnsafe` (- (`self.GravityPullOrigin`) (`self.K2_GetActorLocation`))) (`self.GravityPullIntensity`) false)))))

(event `EnhancedInput|/Game/Jet/Input/Inputs/IA_Camera`
  (params (ActionValue :type "Vector2D Structure") (ElapsedSeconds :type "Float (double-precision)") (TriggeredSeconds :type "Float (double-precision)") (InputAction :type "InputAction Object Reference" :default "/Game/Jet/Input/Inputs/IA_Camera.IA_Camera"))
  (bind _jetfighter (`self.JetFighter`))
  (:`Triggered`
    (`PrimitiveComponent.AddTorqueInRadians` (`self.JetFighter`) (+ (* (`SceneComponent.GetUpVector` _jetfighter) (`self.TorqueFromInput` ActionValue_X (`self.MaxTorqueYaw`) true)) (* (`SceneComponent.GetRightVector` _jetfighter) (`self.TorqueFromInput` ActionValue_Y (`self.MaxTorquePitch`)))) "None" true)))

(event `EnhancedInput|/Game/Jet/Input/Inputs/IA_Fire`
  (params (ActionValue :type Boolean) (ElapsedSeconds :type "Float (double-precision)") (TriggeredSeconds :type "Float (double-precision)") (InputAction :type "InputAction Object Reference" :default "/Game/Jet/Input/Inputs/IA_Fire.IA_Fire"))
  (:`Triggered`
    (`self.Fire`))
  (:`Started`
    (`self.Fire`)))

(event `EnhancedInput|/Game/Jet/Input/Inputs/IA_UseBonus`
  (params (ActionValue :type Boolean) (ElapsedSeconds :type "Float (double-precision)") (TriggeredSeconds :type "Float (double-precision)") (InputAction :type "InputAction Object Reference" :default "/Game/Jet/Input/Inputs/IA_UseBonus.IA_UseBonus"))
  (:`Triggered`
    (`/Game/Pickable/Components/BC_BonusHolder.UseBonus` (`self.BonusHolder`))))

(event `EnhancedInput|/Game/Jet/Input/Inputs/IA_Roll`
  (params (ActionValue :type "Float (double-precision)") (ElapsedSeconds :type "Float (double-precision)") (TriggeredSeconds :type "Float (double-precision)") (InputAction :type "InputAction Object Reference" :default "/Game/Jet/Input/Inputs/IA_Roll.IA_Roll"))
  (bind _jetfighter (`self.JetFighter`))
  (:`Triggered`
    (bind _output_get (set `self.Action Value Roll` ActionValue))
    (`PrimitiveComponent.AddTorqueInRadians` _jetfighter (* (`SceneComponent.GetForwardVector` _jetfighter) (`self.TorqueFromInput` _output_get (`self.MaxTorqueRoll`))) "None" true)))

(event `self.ReceiveBeginPlay`
  (bind _brush (`Image.Brush` (`/Game/Jet/Blueprints/BW_Interface.Speedlines` (`self.Player HUD`))))
  (`|ExecutionSequence`
    (:`then_0`
      (bind _returnvalue (`|CreateWidget` "/Game/Jet/Blueprints/BW_Interface.BW_Interface_C"))
      (bind _output_get (set `self.Player HUD` _returnvalue))
      (`UserWidget.AddToViewport` _output_get 0)
      (bind _returnvalue_2 (`KismetMaterialLibrary.CreateDynamicMaterialInstance` (`WidgetBlueprintLibrary.GetBrushResourceAsMaterial` _brush)))
      (bind _output_get_2 (set `self.SpeedlinesMaterial` _returnvalue_2))
      (`WidgetBlueprintLibrary.SetBrushResourceToMaterial` _brush _output_get_2)
      (set `self.SpringArmTargetLength` (`SpringArmComponent.TargetArmLength` (`self.SpringArm`)))
      (set `self.ObjectRotation` (`SceneComponent.K2_GetComponentRotation` (`self.JetFighter`)))
      (set `self.FlameScale` (`SceneComponent.K2_GetComponentScale` (`self.Flame`))))
    (:`then_1`
      (`KismetSystemLibrary.K2_SetTimerDelegate` (delegate `Update Speedlines`) 0.01 true)
      (set `self.CameraLagRotation` (`self.K2_GetActorRotation`)))))

(event `Update Speedlines`
  (`self.SpeedlineMaterialValue`))

(event `EnhancedInput|/Game/Jet/Input/Inputs/IA_Vertical`
  (params (ActionValue :type "Float (double-precision)") (ElapsedSeconds :type "Float (double-precision)") (TriggeredSeconds :type "Float (double-precision)") (InputAction :type "InputAction Object Reference" :default "/Game/Jet/Input/Inputs/IA_Vertical.IA_Vertical"))
  (:`Triggered`
    (set `self.MoveUp` (`KismetMathLibrary.SelectFloat` ActionValue -1.0 (> ActionValue 0.0)))))

(event `EnhancedInput|/Game/Jet/Input/Inputs/IA_Turbo`
  (params (ActionValue :type Boolean) (ElapsedSeconds :type "Float (double-precision)") (TriggeredSeconds :type "Float (double-precision)") (InputAction :type "InputAction Object Reference" :default "/Game/Jet/Input/Inputs/IA_Turbo.IA_Turbo"))
  (:`Triggered`
    (`self.HandleTurbo` true))
  (:`Completed`
    (`self.HandleTurbo` false)))

(event `EnhancedInput|/Game/Jet/Input/Inputs/IA_Movement`
  (params (ActionValue :type "Vector2D Structure") (ElapsedSeconds :type "Float (double-precision)") (TriggeredSeconds :type "Float (double-precision)") (InputAction :type "InputAction Object Reference" :default "/Game/Jet/Input/Inputs/IA_Movement.IA_Movement"))
  (bind _returnvalue (`KismetMathLibrary.SelectFloat` -1.0 1.0 (`self.bControlsInverted`)))
  (:`Triggered`
    (set `self.Action Value X` (* ActionValue_X _returnvalue))
    (set `self.Action Value Y` (* ActionValue_Y _returnvalue))
    (`self.AddMovementInput` (`self.GetActorForwardVector`) (`self.Action Value Y`))
    (`self.AddMovementInput` (`self.GetActorRightVector`) (`self.Action Value X`))))

(fn `AutoLevelRoll`
  (params (DeltaTime :type "Float (double-precision)"))
  (bind _returnvalue (`KismetMathLibrary.MakeVector` 0.0 0.0 1.0))
  (bind _jetfighter (`self.JetFighter`))
  (bind _jetfighter_2 (`self.JetFighter`))
  (bind _maxautolevelrolltorque (`self.MaxAutoLevelRollTorque`))
  (bind _returnvalue_2 (`SceneComponent.GetForwardVector` _jetfighter))
  (bind _returnvalue_3 (`KismetMathLibrary.DegAtan2` (`KismetMathLibrary.Dot_VectorVector` (`SceneComponent.GetRightVector` _jetfighter_2) _returnvalue) (`KismetMathLibrary.Dot_VectorVector` (`SceneComponent.GetUpVector` _jetfighter_2) _returnvalue)))
  (bind _returnvalue_4 (< (`KismetMathLibrary.Abs` _returnvalue_3) (`self.RollSmallAngleThreshold`)))
  (if (< (`KismetMathLibrary.Abs` (`self.Action Value Roll`)) (`self.RollInputDeadZone`))
    (`PrimitiveComponent.AddTorqueInRadians` (`self.JetFighter`) (* _returnvalue_2 (`KismetMathLibrary.FClamp` (- (* (* _returnvalue_3 (`KismetMathLibrary.SelectFloat` (`self.RollAutoLevelStrengthSmall`) (`self.RollAutoLevelStrengthLarge`) _returnvalue_4)) -1.0) (* (`KismetMathLibrary.Dot_VectorVector` (`PrimitiveComponent.GetPhysicsAngularVelocityInRadians` _jetfighter "None") _returnvalue_2) (`KismetMathLibrary.SelectFloat` (`self.RollAutoLevelDampingSmall`) (`self.RollAutoLevelDampingLarge`) _returnvalue_4))) (* _maxautolevelrolltorque -1.0) _maxautolevelrolltorque)) "None" true)))

(fn `CalculateSpeedState`
  (returns (SpeedValue :type "Float (double-precision)"))
  (bind _floatingpawnmovement (`self.FloatingPawnMovement`))
  (bind _output_get (set `self.Speed` (`KismetMathLibrary.FInterpTo` (`self.Speed`) (`KismetMathLibrary.MapRangeClamped` (`KismetMathLibrary.VSize` (`MovementComponent.Velocity` _floatingpawnmovement)) 0.0 (`MovementComponent.GetMaxSpeed` _floatingpawnmovement) 0.0 (`KismetMathLibrary.SelectFloat` 2.0 1.0 (`self.isBoost?`))) (`GameplayStatics.GetWorldDeltaSeconds`) 5.0)))
  (return _output_get))

(fn `CameraFollowWithLag`
  (params (DeltaTime :type "Float (double-precision)"))
  (bind _returnvalue (`self.K2_GetActorRotation`))
  (bind _maxcameralagangle (`self.MaxCameraLagAngle`))
  (bind _returnvalue_2 (`KismetMathLibrary.RInterpTo` (`self.CameraLagRotation`) _returnvalue DeltaTime (`self.CameraLagSpeed`)))
  (set `self.CameraLagRotation` _returnvalue_2)
  (`SceneComponent.K2_SetRelativeRotation` (`self.SpringArm`) (`KismetMathLibrary.MakeRotator` 90.0 (+ (`KismetMathLibrary.ClampAngle` (.pitch (`KismetMathLibrary.NormalizedDeltaRotator` _returnvalue _returnvalue_2)) (* _maxcameralagangle -1.0) _maxcameralagangle) -10.0) (`KismetMathLibrary.ClampAngle` (.yaw (`KismetMathLibrary.NormalizedDeltaRotator` _returnvalue _returnvalue_2)) (* _maxcameralagangle -1.0) _maxcameralagangle)) false false))

(fn `ClearFreeze`
  (`self.EnableInput` (`GameplayStatics.GetPlayerController` 0)))

(fn `ClearGravity`
  (set `self.bGravityPull` false))

(fn `ClearInversion`
  (set `self.bControlsInverted` false))

(fn `Fire`
  (`NiagaraFunctionLibrary.SpawnSystemAtLocation` "/Game/Jet/Blueprints/Laser/NF_LaserBeam.NF_LaserBeam"))

(fn `Flame intensity`
  (params (Intensity :type "Float (double-precision)"))
  (bind _intensity (`local.Intensity`))
  (bind _pointlight (`self.PointLight`))
  (bind _flamescale (`self.FlameScale`))
  (`SceneComponent.SetWorldScale3D` (`self.Flame`) (`KismetMathLibrary.VLerp` _flamescale (`KismetMathLibrary.MakeVector` (* (.x _flamescale) 50.0) (.y _flamescale) (.z _flamescale)) _intensity))
  (`LightComponent.SetIntensity` _pointlight (`KismetMathLibrary.Lerp` (`LightComponentBase.Intensity` _pointlight) 50.0 _intensity)))

(fn `HandleTurbo`
  (params (bTurboPressed :type Boolean))
  (set `self.isBoost?` (and (and (> (`self.Action Value X`) 0.0) (== (`self.Action Value Y`) 0.0)) bTurboPressed))
  (`self.Max Speed`))

(fn `Max Speed`
  (bind _floatingpawnmovement (`self.FloatingPawnMovement`))
  (bind _isboost_ (`self.isBoost?`))
  (bind _boostspeed (`self.BoostSpeed`))
  (bind _maxspeed (`self.MaxSpeed`))
  (set `FloatingPawnMovement.MaxSpeed` (`KismetMathLibrary.SelectFloat` _boostspeed _maxspeed _isboost_) _floatingpawnmovement)
  (set `FloatingPawnMovement.Deceleration` (`KismetMathLibrary.SelectFloat` 2000.0 500.0 (not _isboost_)) _floatingpawnmovement)
  (set `FloatingPawnMovement.Acceleration` (`KismetMathLibrary.SelectFloat` (* _boostspeed (`self.BoostMultiplier`)) _maxspeed _isboost_) _floatingpawnmovement))

(fn `ResetFire`
  (set `self.bCanFire` true))

(fn `SmoothCameraAndMovement`
  (set `self.CamPitchCurrent` (`KismetMathLibrary.FInterpTo` (`self.CamPitchCurrent`) (`self.CamPitchTarget`) (`GameplayStatics.GetWorldDeltaSeconds`) (`self.CameraInertiaSpeed`)))
  (set `self.CamYawCurrent` (`KismetMathLibrary.FInterpTo` (`self.CamYawCurrent`) (`self.CamYawTarget`) (`GameplayStatics.GetWorldDeltaSeconds`) (`self.CameraInertiaSpeed`)))
  (`self.AddControllerPitchInput` (`self.CamPitchCurrent`))
  (`self.AddControllerYawInput` (`self.CamYawCurrent`))
  (`Controller.SetControlRotation` (`self.GetController`) (`KismetMathLibrary.MakeRotator` 0.0 (`KismetMathLibrary.ClampAngle` (.pitch (`self.GetControlRotation`)) -85.0 85.0) (.yaw (`self.GetControlRotation`)))))

(fn `SpeedlineMaterialValue`
  (bind _speed (`self.Speed`))
  (bind _speedlinesmaterial (`self.SpeedlinesMaterial`))
  (if (> _speed 1.0)
    (`|ExecutionSequence`
      (:`then_0`
        (`MaterialInstanceDynamic.SetScalarParameterValue` _speedlinesmaterial "Center Fade" (`KismetMathLibrary.MapRangeClamped` _speed 1.0 1.5 0.6 0.25)))
      (:`then_1`
        (`MaterialInstanceDynamic.SetScalarParameterValue` _speedlinesmaterial "Center Fade Edge" (`KismetMathLibrary.MapRangeClamped` _speed 1.0 1.5 0.8 0.25)))
      (:`then_2`
        (`MaterialInstanceDynamic.SetScalarParameterValue` _speedlinesmaterial "Line Density" (`KismetMathLibrary.MapRangeClamped` _speed 1.0 1.5 0.0 1.0)))
      (:`then_3`
        (`MaterialInstanceDynamic.SetScalarParameterValue` _speedlinesmaterial "Line Falloff" (`KismetMathLibrary.MapRangeClamped` _speed 1.0 1.5 2.0 0.8)))
      (:`then_4`
        (`MaterialInstanceDynamic.SetScalarParameterValue` _speedlinesmaterial "Line Scale X" (`KismetMathLibrary.MapRangeClamped` _speed 1.0 1.5 2.0 0.9)))
      (:`then_5`
        (`MaterialInstanceDynamic.SetScalarParameterValue` _speedlinesmaterial "Line Speed X" (`KismetMathLibrary.MapRangeClamped` _speed 1.0 1.5 1.5 4.0)))
      (:`then_6`
        (`MaterialInstanceDynamic.SetScalarParameterValue` _speedlinesmaterial "Opacity" (`KismetMathLibrary.MapRangeClamped` _speed 1.0 1.5 0.0 0.5)))
      (:`then_7`
        (`MaterialInstanceDynamic.SetScalarParameterValue` _speedlinesmaterial "Saturation Color" (`KismetMathLibrary.MapRangeClamped` _speed 1.0 1.5 0.0 0.7))))))

(fn `SpringArmLengthInterpolation`
  (bind _springarm (`self.SpringArm`))
  (bind _springarmtargetlength (`self.SpringArmTargetLength`))
  (bind _camera (`self.Camera`))
  (set `self.isMoving?` (> (`self.Speed`) 0.01))
  (set `SpringArmComponent.TargetArmLength` (`KismetMathLibrary.FInterpTo` (`SpringArmComponent.TargetArmLength` _springarm) (`KismetMathLibrary.SelectFloat` (`self.SpringArmMaxLength`) (`KismetMathLibrary.FInterpTo` (`KismetMathLibrary.SelectFloat` (* _springarmtargetlength 1.2) _springarmtargetlength (`self.isMoving?`)) (`self.SpringArmTargetLength`) (`GameplayStatics.GetWorldDeltaSeconds`) 2.0) (`self.isBoost?`)) (`GameplayStatics.GetWorldDeltaSeconds`) 1.0) _springarm)
  (`CameraComponent.SetFieldOfView` _camera (`KismetMathLibrary.FInterpTo` (`CameraComponent.FieldOfView` _camera) (`KismetMathLibrary.SelectFloat` 70.0 90.0 (`self.isBoost?`)) (`GameplayStatics.GetWorldDeltaSeconds`) 1.0)))

(fn `TorqueFromInput`
  (params (InputValue :type "Float (double-precision)") (MaxTorque :type "Float (double-precision)") (Inverse :type Boolean))
  (returns (TorqueValue :type "Float (double-precision)"))
  (bind _returnvalue (* (`KismetMathLibrary.FClamp` InputValue -1.0) MaxTorque))
  (return (`KismetMathLibrary.SelectFloat` (* _returnvalue -1.0) _returnvalue Inverse)))

(fn `UserConstructionScript`)