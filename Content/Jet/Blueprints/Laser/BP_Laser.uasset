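; BP_Laser is a short-lived laser actor that detects what lies along its forward axis and destroys itself after a set Duration.
; Each Tick runs CollisionDetection, a Visibility line trace from the actor's location with its length derived from the X scale.
; On a hit it stores the impact point, actor and component, but applies no damage or effects here.
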(event `self.ReceiveBeginPlay`
  (`KismetSystemLibrary.Delay` (`self.Duration`))
  (`/Engine/EditorBlueprintResources/StandardMacros.IsValid` self
    (:`Is Valid`
      (`self.K2_DestroyActor`))))

(event `self.ReceiveTick`
  (params (DeltaSeconds :type "Float (single-precision)"))
  (`self.CollisionDetection`))

(fn `CollisionDetection`
  (bind _returnvalue (`self.K2_GetActorLocation`))
  (bind (_outhit _returnvalue_2) (`KismetSystemLibrary.LineTraceSingle` _returnvalue (+ _returnvalue (* (`KismetMathLibrary.GetForwardVector` (`self.K2_GetActorRotation`)) (* (.x (`self.GetActorScale3D`)) 200.0))) "TraceTypeQuery1"))
  (if _returnvalue_2
    (bind (_bblockinghit _binitialoverlap _time _distance _location _impactpoint _normal _impactnormal _physmat _hitactor _hitcomponent) (`GameplayStatics.BreakHitResult` _outhit))
    (set `self.Impact Point` _impactpoint)
    (set `self.Hit Actor` _hitactor)
    (set `self.Hit Component` _hitcomponent)))

(fn `UserConstructionScript`)