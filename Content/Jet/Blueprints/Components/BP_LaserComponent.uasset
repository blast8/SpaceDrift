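; Laser weapon component for the Jet game that deals instant hit-scan damage to actors with health.
; Fire, gated by CanFire, runs a Visibility line trace from the component along its local X axis out to LaserRange.
; A hit on an actor with BP_HealthSystem applies Laser-sourced damage and starts the cooldown timer that restores CanFire.
; Any other shot leaves CanFire false, since no timer starts.
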(event `OnCooldownReset`
  (set `self.bCanFire` true))

(fn `Fire`
  (if (`self.bCanFire`)
    (set `self.bCanFire` false)
    (bind (_outhit _returnvalue) (`KismetSystemLibrary.LineTraceSingle` (`self.K2_GetComponentLocation`) (`KismetMathLibrary.TransformLocation` (`self.K2_GetComponentToWorld`) (`KismetMathLibrary.MakeVector` (`self.LaserRange`))) "TraceTypeQuery1"))
    (if _returnvalue
      (bind (_bblockinghit _binitialoverlap _time _distance _location _impactpoint _normal _impactnormal _physmat _hitactor) (`GameplayStatics.BreakHitResult` _outhit))
      (if (`KismetSystemLibrary.IsValid` _hitactor)
        (bind _returnvalue_2 (`Actor.GetComponentByClass` _hitactor "/Game/Jet/Blueprints/Components/BP_HealthSystem.BP_HealthSystem_C"))
        (if (`KismetSystemLibrary.IsValid` _returnvalue_2)
          (`/Game/Jet/Blueprints/Components/BP_HealthSystem.ApplyDamageBySource` _returnvalue_2 (`self.Damage`) "Laser")
          (`KismetSystemLibrary.K2_SetTimer` null "OnCooldownReset" (`self.FireCooldown`)))))))