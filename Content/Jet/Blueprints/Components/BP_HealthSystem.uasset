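; Health component for the Jet game that tracks health, death and a Healthy/Damaged/Critical/Dead state from percent thresholds.
; BeginPlay resets health to a fixed maximum; damage and healing clamp it, refresh state and fire event dispatchers.
; Damage branches are hardwired true, so invulnerability, CanTakeDamage and source checks only affect reported damage, not health loss.
; Source-based damage passes through unscaled, as the multiplier math is unconnected.
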(event `self.ReceiveBeginPlay`
  (`self.InitializeHealth`))

(fn `ApplyDamage`
  (params (DamageAmount :type "Float (double-precision)"))
  (returns (ActualDamage :type "Float (double-precision)") (bKilled :type Boolean))
  (bind _maxhealth (`self.MaxHealth`))
  (bind _currenthealth (`self.CurrentHealth`))
  (bind _returnvalue (`KismetMathLibrary.FClamp` (- _currenthealth DamageAmount) 0.0 _maxhealth))
  (bind _returnvalue_2 (`KismetMathLibrary.InRange_FloatFloat` _returnvalue 0.0 0.0))
  (bind _returnvalue_3 (- _currenthealth _returnvalue))
  (if true
    (bind _output_get (set `self.CurrentHealth` _returnvalue))
    (`self.OnDamaged` _returnvalue_3 _output_get)
    (`self.UpdateHealthState`)
    (`self.OnHealthChanged` _currenthealth _maxhealth (`self.GetHealthPercent`))
    (`self.OnStateChanged` (`self.HealthState`))
    (if _returnvalue_2
      (`self.Kill`)))
  (return (`KismetMathLibrary.SelectFloat` _returnvalue_3 0.0 (and (and (`self.bCanTakeDamage`) (not (`self.bIsDead`))) (not (`self.bInvulnerable`)))) (or (`self.bIsDead`) _returnvalue_2)))

(fn `ApplyDamageBySource`
  (params (DamageAmount :type "Float (double-precision)") (DamageSource :type Name))
  (returns (ActualDamage :type "Float (double-precision)") (bKilled :type Boolean))
  (bind (_resolveddamage _bcanaffecthealth) (`self.ResolveDamageBySource` DamageAmount DamageSource))
  (if true
    (bind (_actualdamage _bkilled) (`self.ApplyDamage` _resolveddamage)))
  (return (`KismetMathLibrary.SelectFloat` _actualdamage 0.0 (and (and (and (`self.bCanTakeDamage`) (not (`self.bInvulnerable`))) (`KismetMathLibrary.InRange_FloatFloat` _resolveddamage (`self.MinDamageThreshold`) 99999.0)) _bcanaffecthealth)) (or _bkilled (`self.bIsDead`))))

(fn `ApplyHeal`
  (params (HealAmount :type "Float (double-precision)"))
  (returns (ActualHeal :type "Float (double-precision)"))
  (bind _currenthealth (`self.CurrentHealth`))
  (bind _returnvalue (not (`self.bIsDead`)))
  (bind _returnvalue_2 (`KismetMathLibrary.FClamp` (+ _currenthealth (`KismetMathLibrary.FClamp` HealAmount 0.0 (`self.MaxHealth`))) 0.0 (`self.MaxHealth`)))
  (if _returnvalue
    (set `self.CurrentHealth` _returnvalue_2)
    (`self.UpdateHealthState`)
    (`self.OnHealthChanged` _returnvalue_2 (`self.MaxHealth`) (`self.GetHealthPercent`))
    (`self.OnStateChanged` (`self.HealthState`)))
  (return (`KismetMathLibrary.SelectFloat` (- _returnvalue_2 _currenthealth) 0.0 _returnvalue)))

(fn `GetHealthPercent`
  (returns (HealthPercent :type "Float (double-precision)"))
  (return (* (`KismetMathLibrary.SafeDivide` (`self.CurrentHealth`) (`self.MaxHealth`)) 100.0)))

(fn `InitializeHealth`
  (set `self.MaxHealth` 100.0)
  (set `self.bIsDead` false)
  (set `self.CurrentHealth` (`self.MaxHealth`))
  (`self.UpdateHealthState`))

(fn `IsAlive`
  (returns (ReturnValue :type Boolean))
  (return (not (`self.bIsDead`))))

(fn `Kill`
  (set `self.CurrentHealth` 0.0)
  (set `self.bIsDead` true)
  (set `self.HealthState` "Dead")
  (`self.OnDeath`))

(fn `ResolveDamageBySource`
  (params (DamageAmount :type "Float (double-precision)") (DamageSource :type Name))
  (returns (ResolvedDamage :type "Float (double-precision)") (bCanAffectHealth :type Boolean))
  (bind _returnvalue (`KismetStringLibrary.Conv_NameToString` DamageSource))
  (return DamageAmount (or (or (`KismetStringLibrary.EqualEqual_StrStr` _returnvalue "Projectile") (`KismetStringLibrary.EqualEqual_StrStr` _returnvalue "Collision")) (or (`KismetStringLibrary.EqualEqual_StrStr` _returnvalue "Environment") (`KismetStringLibrary.EqualEqual_StrStr` _returnvalue "Unknown")))))

(fn `UpdateHealthState`
  (bind _healthpercent (`self.GetHealthPercent`))
  (if (or (`self.bIsDead`) (`KismetMathLibrary.InRange_FloatFloat` _healthpercent -999999.0 0.0))
    (set `self.bIsDead` true)
    (set `self.HealthState` "Dead")
    (elif (`KismetMathLibrary.InRange_FloatFloat` _healthpercent 0.0 (`self.CriticalStateThreshold`) false)
      (set `self.bIsDead` false)
      (set `self.HealthState` "Critical")
      (elif (`KismetMathLibrary.InRange_FloatFloat` _healthpercent (`self.CriticalStateThreshold`) (`self.HealthyStateThreshold`) false)
        (set `self.bIsDead` false)
        (set `self.HealthState` "Damaged")
        (else
          (set `self.bIsDead` false)
          (set `self.HealthState` "Healthy"))))))