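; Shield component for its owning actor that absorbs damage, returning absorbed and overflow amounts, and regenerates over time.
; Tick restores shield at a set rate once a delay since the last hit passes, even from broken, if regeneration is allowed and the shield is active.
; An optional BP_ShieldSphere is spawned attached to the owner and hidden while inactive or broken.
; GetShieldPercent's calculation is unwired, so it never runs.
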(event `self.ReceiveBeginPlay`
  (`|ExecutionSequence`
    (:`then_0`
      (if (`self.AutoInitializeOnBeginPlay`)
        (`self.InitializeShield`)))
    (:`then_1`
      (`self.SpawnShieldVisual`))))

(event `self.ReceiveTick`
  (params (DeltaSeconds :type "Float (single-precision)"))
  (`self.UpdateShieldRegeneration` DeltaSeconds))

(fn `ApplyShieldDamage`
  (params (DamageAmount :type "Float (double-precision)"))
  (returns (OverflowDamage :type "Float (double-precision)") (AbsorbedDamage :type "Float (double-precision)"))
  (bind _currentshield (`self.CurrentShield`))
  (bind _returnvalue (`KismetMathLibrary.FMin` DamageAmount _currentshield))
  (bind _returnvalue_2 (`KismetMathLibrary.FMax` (- _currentshield _returnvalue)))
  (if (and (and (`self.bShieldActive`) (> DamageAmount 0.0)) (> _currentshield 0.0))
    (set `self.CurrentShield` _returnvalue_2)
    (set `self.LastDamageTime` (`KismetSystemLibrary.GetGameTimeInSeconds`))
    (set `self.bShieldBroken` (<= _returnvalue_2 0.0))
    (`self.UpdateShieldVisual`)
    (return (`KismetMathLibrary.FMax` (- DamageAmount _returnvalue)) _returnvalue)
    (else
      (return (`KismetMathLibrary.FMax` DamageAmount) 0.0))))

(fn `CanStartRegenerating`
  (returns (CanRegenerateNow :type Boolean))
  (return (and (and (and (`self.bCanRegenerate`) (`self.bShieldActive`)) (< (`self.CurrentShield`) (`self.MaxShield`))) (>= (- (`KismetSystemLibrary.GetGameTimeInSeconds`) (`self.LastDamageTime`)) (`self.ShieldRegenDelay`)))))

(fn `GetShieldPercent`
  (returns (ShieldPercent :type "Float (double-precision)")))

(fn `InitializeShield`
  (set `self.CurrentShield` (`self.MaxShield`))
  (set `self.bShieldBroken` false)
  (set `self.LastDamageTime` -1000.0))

(fn `RestoreShield`
  (params (RestoreAmount :type "Float (double-precision)"))
  (returns (ActualRestored :type "Float (double-precision)"))
  (bind _currentshield (`self.CurrentShield`))
  (bind _maxshield (`self.MaxShield`))
  (bind _returnvalue (`KismetMathLibrary.FMin` (`KismetMathLibrary.FMax` RestoreAmount) (`KismetMathLibrary.FMax` (- _maxshield _currentshield))))
  (bind _returnvalue_2 (`KismetMathLibrary.FClamp` (+ _currentshield _returnvalue) 0.0 _maxshield))
  (set `self.CurrentShield` _returnvalue_2)
  (set `self.bShieldBroken` (<= _returnvalue_2 0.0))
  (`self.UpdateShieldVisual`)
  (return _returnvalue))

(fn `SpawnShieldVisual`
  (bind _returnvalue (`self.GetOwner`))
  (if (`self.bSpawnShieldVisual`)
    (bind _returnvalue_2 (`|SpawnActorFromClass` "/Game/Jet/Blueprints/Components/BP_ShieldSphere.BP_ShieldSphere_C" (`Actor.GetTransform` _returnvalue) "Undefined" "MultiplyWithRoot" _returnvalue null))
    (set `self.ShieldVisualActor` _returnvalue_2)
    (`Actor.K2_AttachToActor` _returnvalue_2 (`self.GetOwner`) "None" "KeepWorld" "KeepWorld" "KeepWorld" true)
    (`Actor.SetActorScale3D` _returnvalue_2 (`self.ShieldVisualScale`))
    (`self.UpdateShieldVisual`)))

(fn `UpdateShieldRegeneration`
  (params (DeltaTime :type "Float (double-precision)"))
  (if (`self.CanStartRegenerating`)
    (`self.RestoreShield` (* (`self.ShieldRegenRate`) DeltaTime))))

(fn `UpdateShieldVisual`
  (`Actor.SetActorHiddenInGame` (`self.ShieldVisualActor`) (or (not (`self.bShieldActive`)) (`self.bShieldBroken`))))